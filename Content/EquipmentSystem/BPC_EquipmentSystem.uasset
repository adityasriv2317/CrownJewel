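; BPC_EquipmentSystem is a component for BP_ThirdPersonCharacter that handles weapon pickup and the equipment menu.
; Interact input sphere-traces forward from the follow camera, stores a hit BP_Weapons' item data in WeaponSlot, then destroys the actor.
; Menu input captures the character's SceneCapture2D, then toggles WB_EquipmentPanel along with cursor and input mode.
; Movement is disabled while the panel is open, and the previous movement mode is restored on close.
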(event `self.ReceiveBeginPlay`
  ;[1 1 1] Get Camera Variable
  (bind _asbp_third_person_character (cast `/Game/ThirdPerson/Blueprints/BP_ThirdPersonCharacter` (`self.GetOwner`)))
  (set `self.Player_Camera` (`/Game/ThirdPerson/Blueprints/BP_ThirdPersonCharacter.FollowCamera` _asbp_third_person_character)))

(event `EnhancedInput|/Game/ThirdPerson/Input/Actions/IA_Interact`
  (params (ActionValue :type Boolean) (ElapsedSeconds :type "Float (double-precision)") (TriggeredSeconds :type "Float (double-precision)") (InputAction :type "InputAction Object Reference" :default "/Game/ThirdPerson/Input/Actions/IA_Interact.IA_Interact"))
  (bind _player_camera (`self.Player_Camera`))
  (bind _returnvalue (`SceneComponent.K2_GetComponentLocation` _player_camera))
  ;[0.05127 0.05127 0.05127] Interaction Detection
  (:`Started`
    (bind (_outhit _returnvalue_2) (`KismetSystemLibrary.SphereTraceSingleForObjects` :`Start` _returnvalue :`End` (+ _returnvalue (* (`KismetMathLibrary.GetForwardVector` (`SceneComponent.K2_GetComponentRotation` _player_camera)) 1000.0)) :`ObjectTypes` (`|MakeArray` "ObjectTypeQuery2" :!type "EObjectTypeQuery Enum") :`DrawDebugType` "ForDuration"))
    (if _returnvalue_2
      (bind _asbp_weapons (cast `/Game/EquipmentSystem/BP_Weapons` (`.HitActor` (`GameplayStatics.BreakHitResult` _outhit))))
      (`self.AddNewWeapon` (`/Game/EquipmentSystem/BP_Weapons.ItemData` _asbp_weapons))
      (`Actor.K2_DestroyActor` _asbp_weapons))))

(event `EnhancedInput|/Game/ThirdPerson/Input/Actions/IA_EquipementMenu`
  (params (ActionValue :type Boolean) (ElapsedSeconds :type "Float (double-precision)") (TriggeredSeconds :type "Float (double-precision)") (InputAction :type "InputAction Object Reference" :default "/Game/ThirdPerson/Input/Actions/IA_EquipementMenu.IA_EquipementMenu"))
  (bind _returnvalue (`GameplayStatics.GetPlayerController` 0))
  (bind _returnvalue_2 (`self.GetOwner`))
  (:`Started`
    (bind _asbp_third_person_character (cast `/Game/ThirdPerson/Blueprints/BP_ThirdPersonCharacter` (`GameplayStatics.GetPlayerCharacter` 0)))
    (`SceneCaptureComponent2D.CaptureScene` (`/Game/ThirdPerson/Blueprints/BP_ThirdPersonCharacter.SceneCaptureComponent2D` _asbp_third_person_character))
    (if (not (`self.is_EqPanel_Open`))
      (set `self.is_EqPanel_Open` true)
      (bind _returnvalue_3 (`|CreateWidget` "/Game/EquipmentSystem/UI/WB_EquipmentPanel.WB_EquipmentPanel_C"))
      (bind _output_get (set `self.PanelWidget` _returnvalue_3))
      (`UserWidget.AddToViewport` _output_get 0)
      (set `PlayerController.bShowMouseCursor` true _returnvalue)
      (`WidgetBlueprintLibrary.SetInputMode_GameAndUIEx` _returnvalue (`self.PanelWidget`))
      (bind _asbp_third_person_character_2 (cast `/Game/ThirdPerson/Blueprints/BP_ThirdPersonCharacter` _returnvalue_2))
      (bind _charactermovement (`Character.CharacterMovement` _asbp_third_person_character_2))
      (set `self.Prev_Movement_Mode` (`CharacterMovementComponent.MovementMode` _charactermovement))
      (`CharacterMovementComponent.SetMovementMode` _charactermovement "MOVE_None" 0)
      (else
        (bind _panelwidget (`self.PanelWidget`)
          (:`then`
            (`Widget.RemoveFromParent` _panelwidget)
            (set `self.PanelWidget` null)
            (set `self.is_EqPanel_Open` false)
            (set `PlayerController.bShowMouseCursor` false _returnvalue)
            (`WidgetBlueprintLibrary.SetInputMode_GameOnly` _returnvalue)
            (bind _asbp_third_person_character_3 (cast `/Game/ThirdPerson/Blueprints/BP_ThirdPersonCharacter` _returnvalue_2))
            (`CharacterMovementComponent.SetMovementMode` (`Character.CharacterMovement` _asbp_third_person_character_3) (`self.Prev_Movement_Mode`) 0))
          (:`else`))))))

(fn `AddNewWeapon`
  (params (NewItem :type "/Game/EquipmentSystem/S_ItemSlots Structure (by ref)"))
  (`KismetArrayLibrary.Array_Add` (`self.Weapon_Slot`) NewItem))