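; Player stats component that tracks health, stamina, XP and level for the owning BP_ThirdPersonCharacter, cached one tick after BeginPlay.
; Health and stamina functions cap gains at maximum, refill on max increases and push percentages straight to the character's HUD bars.
; TakeDamage and UseStamina return true when their pool is depleted.
; Reaching MaxXP discards overflow and calls IncreaseLevel, which raises MaxXP but resets Level to zero after incrementing it.
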(event `self.ReceiveBeginPlay`
  (`KismetSystemLibrary.DelayUntilNextTick`)
  (bind _asbp_third_person_character (cast `/Game/ThirdPerson/Blueprints/BP_ThirdPersonCharacter` (`self.GetOwner`)))
  (set `self.Player_BP` _asbp_third_person_character))

(fn `GetXP`
  (params (A :type "Float (double-precision)"))
  (bind _returnvalue (+ A (`self.XP`)))
  (if (>= _returnvalue (`self.Max XP`))
    (`self.IncreaseLevel`)
    (set `self.XP` 0.0)
    (else
      (set `self.XP` _returnvalue))))

(fn `IncreaseHealth`
  (params (Health :type "Float (double-precision)"))
  (bind _maxhealth (`self.MaxHealth`))
  (bind _returnvalue (+ Health (`self.CurrentHealth`)))
  (if (>= _returnvalue _maxhealth)
    (set `self.CurrentHealth` _maxhealth)
    (else
      (set `self.CurrentHealth` _returnvalue)))
  (`ProgressBar.SetPercent` (`/Game/UI/WB_HUD.HaelthBar` (`/Game/ThirdPerson/Blueprints/BP_ThirdPersonCharacter.HUD_Widget` (`self.Player_BP`))) (/ (`self.CurrentHealth`) _maxhealth)))

(fn `IncreaseLevel`
  (`/Engine/EditorBlueprintResources/StandardMacros.IncrementInt` (`self.Level`)
    (:`  `
      (set `self.Level` 0)
      (set `self.Max XP` (+ (`self.Max XP`) 150.0)))))

(fn `IncreaseMaxStamina`
  (params (A :type "Float (double-precision)"))
  (bind _output_get (set `self.MaxStamina` (+ A (`self.MaxStamina`))))
  (bind _output_get_2 (set `self.CurrentStamina` _output_get))
  (`ProgressBar.SetPercent` (`/Game/UI/WB_HUD.StaminaBar` (`/Game/ThirdPerson/Blueprints/BP_ThirdPersonCharacter.HUD_Widget` (`self.Player_BP`))) (/ _output_get_2 _output_get)))

(fn `IncreaseStamina`
  (params (Stamina :type "Float (double-precision)"))
  (bind _maxstamina (`self.MaxStamina`))
  (bind _returnvalue (+ Stamina (`self.CurrentStamina`)))
  (if (>= _returnvalue _maxstamina)
    (set `self.CurrentStamina` _maxstamina)
    (else
      (set `self.CurrentStamina` _returnvalue)))
  (`ProgressBar.SetPercent` (`/Game/UI/WB_HUD.StaminaBar` (`/Game/ThirdPerson/Blueprints/BP_ThirdPersonCharacter.HUD_Widget` (`self.Player_BP`))) (/ (`self.CurrentStamina`) _maxstamina)))

(fn `TakeDamage`
  (params (Damage :type "Float (double-precision)"))
  (returns (isPlayerDead :type Boolean))
  (bind _currenthealth (`self.CurrentHealth`))
  (if (not (<= _currenthealth 0.0))
    (bind _output_get (set `self.CurrentHealth` (- _currenthealth Damage)))
    (`ProgressBar.SetPercent` (`/Game/UI/WB_HUD.HaelthBar` (`/Game/ThirdPerson/Blueprints/BP_ThirdPersonCharacter.HUD_Widget` (`self.Player_BP`))) (/ _output_get (`self.MaxHealth`)))
    (if (<= _output_get 0.0)
      (set `self.CurrentHealth` 0.0)
      (else
        (return false))))
  (return true))

(fn `UpdateMaxHealth`
  (params (NewMaxHealth :type "Float (double-precision)"))
  (bind _output_get (set `self.MaxHealth` (+ (`self.MaxHealth`) NewMaxHealth)))
  (bind _output_get_2 (set `self.CurrentHealth` _output_get))
  (`ProgressBar.SetPercent` (`/Game/UI/WB_HUD.HaelthBar` (`/Game/ThirdPerson/Blueprints/BP_ThirdPersonCharacter.HUD_Widget` (`self.Player_BP`))) (/ _output_get_2 _output_get)))

(fn `UseStamina`
  (params (Stamina :type "Float (double-precision)"))
  (returns (Drained :type Boolean))
  (bind _currentstamina (`self.CurrentStamina`))
  (if (not (<= _currentstamina 0.0))
    (bind _output_get (set `self.CurrentStamina` (- _currentstamina Stamina)))
    (`ProgressBar.SetPercent` (`/Game/UI/WB_HUD.StaminaBar` (`/Game/ThirdPerson/Blueprints/BP_ThirdPersonCharacter.HUD_Widget` (`self.Player_BP`))) (/ _output_get (`self.MaxStamina`)))
    (if (<= (`self.CurrentStamina`) 0.0)
      (set `self.CurrentStamina` 0.0)
      (else
        (return false))))
  (return true))

(fn `UseXP`
  (params (XP :type "Float (double-precision)"))
  (set `self.XP` (- XP (`self.XP`)))
  (if (<= (`self.XP`) 0.0)
    (set `self.XP` 0.0)))