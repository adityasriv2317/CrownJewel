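; Stats component for BP_Dummy that tracks health, XP and level, caching its owner one tick after BeginPlay.
; Health functions raise the maximum with a full refill, heal up to that cap or apply damage, updating the dummy's health bar.
; TakeDamage returns true once health is depleted, switching the mesh to physics simulation on the killing hit.
; GetXP levels up at MaxXP, resetting XP without carrying overflow and raising the next threshold.
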(event `self.ReceiveBeginPlay`
  (`KismetSystemLibrary.DelayUntilNextTick`)
  (bind _asbp_dummy (cast `/Game/Blueprints/BP_Dummy` (`self.GetOwner`)))
  (set `self.Dummy_BP` _asbp_dummy))

(fn `GetXP`
  (params (A :type "Float (double-precision)"))
  (bind _returnvalue (+ A (`self.XP`)))
  (if (>= _returnvalue (`self.Max XP`))
    (`self.IncreaseLevel`)
    (set `self.XP` 0.0)
    (else
      (set `self.XP` _returnvalue))))

(fn `IncreaseHealth`
  (params (Health :type "Float (double-precision)"))
  (bind _maxhealth (`self.MaxHealth`))
  (bind _returnvalue (+ Health (`self.CurrentHealth`)))
  (if (>= _returnvalue _maxhealth)
    (set `self.CurrentHealth` _maxhealth)
    (else
      (set `self.CurrentHealth` _returnvalue)))
  (`ProgressBar.SetPercent` (`/Game/UI/WB_DummyHealth.HealthBar` (`/Game/Blueprints/BP_Dummy.Dummy_Health_Bar` (`self.Dummy_BP`))) (/ (`self.CurrentHealth`) _maxhealth)))

(fn `IncreaseLevel`
  (bind _result (`/Engine/EditorBlueprintResources/StandardMacros.IncrementInt` (`self.Level`))
    (:`  `
      (set `self.Level` _result)
      (set `self.Max XP` (+ (`self.Max XP`) 150.0)))))

(fn `TakeDamage`
  (params (Damage :type "Float (double-precision)"))
  (returns (isPlayerDead :type Boolean))
  (bind _currenthealth (`self.CurrentHealth`))
  (if (not (<= _currenthealth 0.0))
    (bind _output_get (set `self.CurrentHealth` (- _currenthealth Damage)))
    (`ProgressBar.SetPercent` (`/Game/UI/WB_DummyHealth.HealthBar` (`/Game/Blueprints/BP_Dummy.Dummy_Health_Bar` (`self.Dummy_BP`))) (/ _output_get (`self.MaxHealth`)))
    (if (<= _output_get 0.0)
      (set `self.CurrentHealth` 0.0)
      (`PrimitiveComponent.SetSimulatePhysics` (`Character.Mesh` (`self.Dummy_BP`)) true)
      (else
        (return false))))
  (return true))

(fn `UpdateMaxHealth`
  (params (NewMaxHealth :type "Float (double-precision)"))
  (bind _output_get (set `self.MaxHealth` (+ (`self.MaxHealth`) NewMaxHealth)))
  (bind _output_get_2 (set `self.CurrentHealth` _output_get))
  (`ProgressBar.SetPercent` (`/Game/UI/WB_DummyHealth.HealthBar` (`/Game/Blueprints/BP_Dummy.Dummy_Health_Bar` (`self.Dummy_BP`))) (/ _output_get_2 _output_get)))

(fn `UseXP`
  (params (XP :type "Float (double-precision)"))
  (set `self.XP` (- XP (`self.XP`)))
  (if (<= (`self.XP`) 0.0)
    (set `self.XP` 0.0)))