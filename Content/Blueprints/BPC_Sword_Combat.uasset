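; Sword combat component for the third-person character, running a four-step melee combo of sword swings and a kick.
; Attack input plays montages by combo index or buffers the next hit, which SwordAttackCombo continues or resets.
; Input also starts a looping timer that sphere-traces along the blade, while a separate event traces the kick.
; Hits on "damageable"-tagged actors apply damage, sounds, blood and camera shake, with blade hits throttled by a delayed DoOnce.
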(event `self.ReceiveBeginPlay`
  ;[0.05127 0.05127 0.05127] Cast Variables
  (bind _asbp_third_person_character (cast `/Game/ThirdPerson/Blueprints/BP_ThirdPersonCharacter` (`self.GetOwner`)))
  (set `self.CharacterBP` _asbp_third_person_character)
  (set `self.CharacterMesh` (`Character.Mesh` _asbp_third_person_character)))

(event `EnhancedInput|/Game/ThirdPerson/Input/Actions/IA_Combat`
  (params (ActionValue :type Boolean) (ElapsedSeconds :type "Float (double-precision)") (TriggeredSeconds :type "Float (double-precision)") (InputAction :type "InputAction Object Reference" :default "/Game/ThirdPerson/Input/Actions/IA_Combat.IA_Combat"))
  ;[0.05127 0.05127 0.05127] Attack Combo System
  ;;[1 1 1] Detect Attack Input
  (:`Started`
    (if (`self.canAttack`)
      (`self.Sword Attack`)
      (`self.Start Sword Trace`))))

(event `Attack 1`
  ;[0.05127 0.05127 0.05127] Attack Combo System
  ;;[0 0.0148 0.05127] Attack 1
  (`/Engine/EditorBlueprintResources/StandardMacros.DoOnce` false :!label _label
    (:`Completed`
      (`KismetSystemLibrary.Delay` 0.1)
      (`|PlayMontage` (`self.CharacterMesh`) "/Game/Characters/RPG_Character/Animation/Combat/Sword_Attack1_Montage.Sword_Attack1_Montage"
        (:`then`
          (set `self.Attack_Index` 1)
          (goto _label :!via `Reset`))))))

(event `Sword Attack`
  ;[0.05127 0.05127 0.05127] Attack Combo System
  ;;[1 1 1] Save Attack Combo State
  (if (`self.isAttacking`)
    (set `self.saveAttack` true)
    (else
      (set `self.isAttacking` true)
      (switch `int` (`self.Attack_Index`) :!label _label_2
        (:`0`
          (`self.Attack 1`))
        (:`1`
          (`self.Attack 2`))
        (:`2`
          (`self.Attack 3`))
        (:`3`
          (`self.Attack 4`))))))

(event `Attack 2`
  ;[0.05127 0.05127 0.05127] Attack Combo System
  ;;[0 0.0148 0.05127] Attack 2
  (`/Engine/EditorBlueprintResources/StandardMacros.DoOnce` false :!label _label_3
    (:`Completed`
      (`KismetSystemLibrary.Delay` 0.1)
      (`|PlayMontage` (`self.CharacterMesh`) "/Game/Characters/RPG_Character/Animation/Combat/Sword_Attack2_Montage.Sword_Attack2_Montage"
        (:`then`
          (set `self.Attack_Index` 2)
          (goto _label_3 :!via `Reset`))))))

(event `Sword Attack Combo`
  ;[0.05127 0.05127 0.05127] Attack Combo System
  ;;[1 1 1] If Combo is to be Continued
  (if (`self.saveAttack`)
    (set `self.saveAttack` false)
    (goto _label_2)
    (else
      (`self.Stop Attack Combo`))))

(event `Attack 3`
  ;[0.05127 0.05127 0.05127] Attack Combo System
  ;;[0 0.0148 0.05127] Attack 3
  (`/Engine/EditorBlueprintResources/StandardMacros.DoOnce` false :!label _label_4
    (:`Completed`
      (`KismetSystemLibrary.Delay` 0.1)
      (`|PlayMontage` (`self.CharacterMesh`) "/Game/Characters/RPG_Character/Animation/Combat/Kick1_Montage.Kick1_Montage"
        (:`then`
          (set `self.Attack_Index` 3)
          (goto _label_4 :!via `Reset`))))))

(event `Stop Attack Combo`
  ;[0.05127 0.05127 0.05127] Attack Combo System
  ;;[1 1 1] Stop Attack Combo
  (set `self.isAttacking` false)
  (set `self.Attack_Index` 0))

(event `Attack 4`
  ;[0.05127 0.05127 0.05127] Attack Combo System
  ;;[0 0.0148 0.05127] Attack 4
  (`/Engine/EditorBlueprintResources/StandardMacros.DoOnce` false :!label _label_5
    (:`Completed`
      (`KismetSystemLibrary.Delay` 0.1)
      (`|PlayMontage` (`self.CharacterMesh`) "/Game/Characters/RPG_Character/Animation/Combat/Sword_Attack3_Montage.Sword_Attack3_Montage"
        (:`then`
          (set `self.Attack_Index` 4)
          (goto _label_5 :!via `Reset`))))))

(event `Start Sword Trace`
  ;[0.05127 0.05127 0.05127] Sword Tace and Damage
  (bind _returnvalue (`KismetSystemLibrary.K2_SetTimerDelegate` (delegate `Sword Trace Loop`) 0.01 true))
  (set `self.SwordTraceLoop` _returnvalue))

(event `SphereTrace`
  (bind _returnvalue (`SceneComponent.K2_GetComponentLocation` (`/Game/ThirdPerson/Blueprints/BP_ThirdPersonCharacter.Kick_SphereTrace` (`self.CharacterBP`))))
  ;[0.05127 0.05127 0.05127] SphereTrace Kick Damage
  (bind (_outhit _returnvalue_2) (`KismetSystemLibrary.SphereTraceSingle` :`Start` _returnvalue :`End` _returnvalue :`Radius` 25.0 :`TraceChannel` "TraceTypeQuery1" :`TraceColor` (struct :`R` 0.120417 :`G` 1.0 :`A` 1.0) :`DrawTime` 0.5))
  (if _returnvalue_2
    (bind (_bblockinghit _binitialoverlap _time _distance _location _impactpoint _normal _impactnormal _physmat _hitactor) (`GameplayStatics.BreakHitResult` _outhit))
    (if (`Actor.ActorHasTag` _hitactor "damageable")
      (`GameplayStatics.ApplyDamage` _hitactor 35.0)
      (`GameplayStatics.PlayWorldCameraShake` "/Game/Blueprints/BP_Sword_CameraShake.BP_Sword_CameraShake_C" _location 0.0 5000.0)
      (`self.Play Hit Sounds`)
      (`GameplayStatics.SpawnEmitterAtLocation` "/Game/Effects/Particles/Blood/P_Blood_Splat_Cone.P_Blood_Splat_Cone" _location (`KismetMathLibrary.MakeRotFromXY` _normal _normal) (0.4 1.0 1.0) true "AutoRelease"))))

(event `Sword Trace Loop`
  (bind _characterbp (`self.CharacterBP`))
  ;[0.05127 0.05127 0.05127] Sword Tace and Damage
  (bind (_outhit _returnvalue) (`KismetSystemLibrary.SphereTraceSingle` :`Start` (`SceneComponent.K2_GetComponentLocation` (`/Game/ThirdPerson/Blueprints/BP_ThirdPersonCharacter.Sword_Tip` _characterbp)) :`End` (`SceneComponent.K2_GetComponentLocation` (`/Game/ThirdPerson/Blueprints/BP_ThirdPersonCharacter.Sword_Blade` _characterbp)) :`Radius` 12.0 :`TraceChannel` "TraceTypeQuery1" :`DrawTime` 0.1))
  (if _returnvalue
    (bind (_bblockinghit _binitialoverlap _time _distance _location _impactpoint _normal _impactnormal _physmat _hitactor) (`GameplayStatics.BreakHitResult` _outhit))
    (if (`Actor.ActorHasTag` _hitactor "damageable")
      (`/Engine/EditorBlueprintResources/StandardMacros.DoOnce` false :!label _label_6
        (:`Completed`
          (`GameplayStatics.ApplyDamage` _hitactor 15.0)
          (`self.Play Hit Sounds`)
          (`GameplayStatics.SpawnEmitterAtLocation` "/Game/Effects/Particles/Blood/P_Blood_Splat_Cone.P_Blood_Splat_Cone" _location (`KismetMathLibrary.MakeRotFromXY` _normal _normal) (0.4 1.0 1.0) true "AutoRelease")
          (`GameplayStatics.PlayWorldCameraShake` "/Game/Blueprints/BP_Sword_CameraShake.BP_Sword_CameraShake_C" _location 0.0 5000.0)
          (`KismetSystemLibrary.Delay` 0.5)
          (goto _label_6 :!via `Reset`))))))

(event `Stop Sword Trace`
  ;[0.05127 0.05127 0.05127] Sword Tace and Damage
  (`KismetSystemLibrary.K2_ClearAndInvalidateTimerHandle` (`self.SwordTraceLoop`)))

(event `Play Hit Sounds`
  (bind _returnvalue (`Actor.K2_GetActorLocation` (`self.GetOwner`)))
  ;[1 1 1] Sword Hit Sounds
  (`GameplayStatics.PlaySoundAtLocation` "/Game/Audio/Sword_Hit/Hit1.Hit1" _returnvalue (struct) 1.0 1.0 0.0 null null null null)
  (`GameplayStatics.PlaySoundAtLocation` "/Game/Audio/Sword_Hit/Hit2.Hit2" _returnvalue (struct) 1.0 1.0 0.0 null null null null))