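; Dummy character that serves as a victim for the player's stealth back-attack assassination.
; AssassinRadius overlaps with the third-person character show and hide the StealthLMB prompt, which rotates every Tick to face the camera.
; StealthBackAttack plays the victim montage, hides the prompt and triggers mesh ragdoll physics after a short random delay.
; It returns the REFAssassinMesh location and the dummy's rotation as a reference transform for the caller.
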(event `self.ReceiveTick`
  (params (DeltaSeconds :type "Float (single-precision)"))
  (`SceneComponent.K2_SetWorldRotation` (`self.stealthLMB`) (`KismetMathLibrary.FindLookAtRotation` (`SceneComponent.K2_GetComponentLocation` (`self.stealthLMB`)) (`SceneComponent.K2_GetComponentLocation` (`PlayerCameraManager.TransformComponent` (`GameplayStatics.GetPlayerCameraManager` 0)))) false false))

(event `Ragdolled`
  ;[0.05127 0.05127 0.05127] Assassination
  (`KismetSystemLibrary.Delay` (`KismetMathLibrary.RandomFloatInRange` 1.9 2.5))
  (`PrimitiveComponent.SetSimulatePhysics` (`self.Mesh`) true))

(event `self.Assassin Radius.OnComponentBeginOverlap`
  (params (OverlappedComponent :type "PrimitiveComponent Object Reference") (OtherActor :type "Actor Object Reference") (OtherComp :type "PrimitiveComponent Object Reference") (OtherBodyIndex :type Integer) (bFromSweep :type Boolean) (SweepResult :type "HitResult Structure (by ref)"))
  ;[0.05127 0.05127 0.05127] Assassination
  (cast `/Game/ThirdPerson/Blueprints/BP_ThirdPersonCharacter` OtherActor)
  (`SceneComponent.SetVisibility` (`self.stealthLMB`) true false))

(event `self.Assassin Radius.OnComponentEndOverlap`
  (params (OverlappedComponent :type "PrimitiveComponent Object Reference") (OtherActor :type "Actor Object Reference") (OtherComp :type "PrimitiveComponent Object Reference") (OtherBodyIndex :type Integer))
  ;[0.05127 0.05127 0.05127] Assassination
  (cast `/Game/ThirdPerson/Blueprints/BP_ThirdPersonCharacter` OtherActor)
  (`SceneComponent.SetVisibility` (`self.stealthLMB`) false false))

(fn `Stealth Back Attack`
  (returns (`Reference Position` :type "Vector Structure") (Rotation :type "Rotator Structure"))
  (`self.PlayAnimMontage` "/Game/Characters/RPG_Character/Animation/Assassinations/AM_Assassinn_Victim.AM_Assassinn_Victim")
  (`self.Ragdolled`)
  (`SceneComponent.SetVisibility` (`self.stealthLMB`) false false)
  (return (`SceneComponent.K2_GetComponentLocation` (`self.REF_AssassinMesh`)) (`self.K2_GetActorRotation`)))

(fn `UserConstructionScript`)